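; BP_ProjectileCheval is a projectile that damages players it hits and reports the hit to the player who fired it.
; Its movement speed is set from the Speed variable in both the construction script and BeginPlay.
; On collision overlap it ignores its instigator, damages a BP_Player, destroys itself, then calls HaveIt on the instigator with the damage as points and the victim's ID and reference.
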(event OnComponentBeginOverlap(Collision)
  (params (OverlappedComponent :type Primitive%20Component%20Object%20Reference) (OtherActor :type Actor%20Object%20Reference) (OtherComp :type Primitive%20Component%20Object%20Reference) (OtherBodyIndex :type Integer) (bFromSweep :type Boolean) (SweepResult :type Hit%20Result%20Structure%20%28by%20ref%29))
  (bind _returnvalue (Game|GetInstigator))
  (if (not (== OtherActor (Game|GetInstigator)))
    (Development|PrintString (Utilities|GetDisplayName OtherActor))
    (bind _asbp_player (Utilities|Casting|CastToBP_Player OtherActor))
    (Game|Damage|ApplyDamage _asbp_player (Variables|Default|GetDamage) 0 0)
    (Actor|DestroyActor)
    (Development|PrintString (Utilities|GetDisplayName _returnvalue) true true "(R=1.000000,G=0.060636,B=0.000000,A=1.000000)")
    (bind _asbp_player_2 (Utilities|Casting|CastToBP_Player _returnvalue))
    (Default|HaveIt _asbp_player_2 (Variables|Default|GetDamage) (Variables|/Game/Player/Blueprints/BP_Player.BP_Player_C|GetPlayer%20ID _asbp_player) _asbp_player)))

(event EventBeginPlay
  (bind _projectilemovement (Variables|Default|GetProjectileMovement))
  (bind _speed (Variables|Default|GetSpeed))
  (Variables|/Script/Engine.ProjectileMovementComponent|SetMaxSpeed _projectilemovement _speed)
  (Variables|/Script/Engine.ProjectileMovementComponent|SetInitialSpeed _projectilemovement _speed))

(event Collision|EventActorBeginOverlap
  (params (OtherActor :type Actor%20Object%20Reference)))

(event EventTick
  (params (DeltaSeconds :type Float%20%28single-precision%29)))

(fn ConstructionScript
  (bind _projectilemovement (Variables|Default|GetProjectileMovement))
  (bind _speed (Variables|Default|GetSpeed))
  (Variables|/Script/Engine.ProjectileMovementComponent|SetMaxSpeed _projectilemovement _speed)
  (Variables|/Script/Engine.ProjectileMovementComponent|SetInitialSpeed _projectilemovement _speed))