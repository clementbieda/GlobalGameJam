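; Player projectile that damages the first other player it touches and credits the shooter.
; Its Speed variable sets the ProjectileMovement initial and max speed in the construction script and again on BeginPlay.
; Each Tick, a zero-length sphere trace at the Arrow looks for Pawns, ignoring itself and its instigator.
; A BP_Player hit takes Damage, the instigating player's HaveIt receives that amount as points, then the projectile destroys itself.
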(event EventBeginPlay
  (bind _projectilemovement (Variables|Default|GetProjectileMovement))
  (bind _speed (Variables|Default|GetSpeed))
  (Variables|/Script/Engine.ProjectileMovementComponent|SetMaxSpeed _projectilemovement _speed)
  (Variables|/Script/Engine.ProjectileMovementComponent|SetInitialSpeed _projectilemovement _speed))

(event Collision|EventActorBeginOverlap
  (params (OtherActor :type Actor%20Object%20Reference)))

(event EventTick
  (params (DeltaSeconds :type Float%20%28single-precision%29))
  (bind _arrow (Variables|Default|GetArrow))
  (bind _returnvalue (Transformation|GetWorldLocation _arrow))
  (bind (_outhit _returnvalue_2) (Collision|SphereTraceForObjects _returnvalue _returnvalue 4e+01 (Utilities|Array|MakeArray "ObjectTypeQuery3") false (Utilities|Array|MakeArray self (Game|GetInstigator)) "None" true "(R=1.000000,G=0.000000,B=0.000000,A=1.000000)" "(R=0.000000,G=1.000000,B=0.000000,A=1.000000)" 1.0))
  (if _returnvalue_2
    (bind _asbp_player (Utilities|Casting|CastToBP_Player (.HitActor (Collision|BreakHitResult _outhit))))
    (Game|Damage|ApplyDamage _asbp_player (Variables|Default|GetDamage) 0 0)
    (bind _asbp_player_2 (Utilities|Casting|CastToBP_Player (Game|GetInstigator)))
    (Default|HaveIt _asbp_player_2 (Variables|Default|GetDamage) (Variables|/Game/Player/Blueprints/BP_Player.BP_Player_C|GetPlayer%20ID _asbp_player) _asbp_player)
    (Actor|DestroyActor)))

(fn ConstructionScript
  (bind _projectilemovement (Variables|Default|GetProjectileMovement))
  (bind _speed (Variables|Default|GetSpeed))
  (Variables|/Script/Engine.ProjectileMovementComponent|SetMaxSpeed _projectilemovement _speed)
  (Variables|/Script/Engine.ProjectileMovementComponent|SetInitialSpeed _projectilemovement _speed))