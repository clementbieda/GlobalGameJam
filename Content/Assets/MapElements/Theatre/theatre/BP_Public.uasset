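; Theatre audience Blueprint that animates its Publix component with idle movement and a laugh motion.
; On BeginPlay, PublicMoving starts the Move1 timeline, which ping-pongs through a FlipFlop on each finish to drive Publix's relative location.
; PublicLaugh alternates playing and reversing the PublicLaughin timeline on the same component, then calls PublicMoving when finished.
; The laugh event does not stop Move1, so both timelines can write the location simultaneously.
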(event Custom|PublicMoving
  (Utilities|FlowControl|FlipFlop :!label _label
    (:A
      (bind _newtrack_0 (Timeline|Move1 Play)
        (:Update
          (Transformation|SetRelativeLocation (Variables|Default|GetPublix) (Math|Vector|MakeVector (.x _newtrack_0) (.y _newtrack_0) (.z _newtrack_0)) false false))
        (:Finished
          (goto _label))))
    (:B
      (Timeline|Move1 Reverse))))

(event Custom|PublicLaugh
  (Utilities|FlowControl|FlipFlop
    (:A
      (bind _newtrack_0 (Timeline|PublicLaughin Play)
        (:Update
          (Transformation|SetRelativeLocation (Variables|Default|GetPublix) (Math|Vector|MakeVector (.x _newtrack_0) (.y _newtrack_0) (.z _newtrack_0)) false false))
        (:Finished
          (CallFunction|PublicMoving))))
    (:B
      (Timeline|PublicLaughin Reverse))))

(event EventBeginPlay
  (CallFunction|PublicMoving))

(event Collision|EventActorBeginOverlap
  (params (OtherActor :type Actor%20Object%20Reference)))

(fn ConstructionScript)