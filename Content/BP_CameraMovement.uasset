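; BP_CameraMovement is a shared two-player camera actor that zooms according to how far both players are from it, with its location treated as the fight zone's middle.
; BeginPlay retries on short delays until player characters 0 and 1 are valid, then caches them.
; Tick smoothly interpolates the SpringArm length toward the scaled sum of both distances, gated by loose minimum and maximum distance checks that either player can satisfy.
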(event EventBeginPlay
  (bind _returnvalue (Game|GetPlayerCharacter 1))
  (bind _returnvalue_2 (Game|GetPlayerCharacter 0))
  (Utilities|FlowControl|Sequence
    (:then_0
      (Utilities|IsValid _returnvalue_2 :!label _label
        (:Is%20Valid
          (Variables|Default|SetPlayer1 _returnvalue_2))
        (:Is%20Not%20Valid
          (Utilities|FlowControl|Delay 0.2)
          (goto _label))))
    (:then_1
      (Utilities|IsValid _returnvalue :!label _label_2
        (:Is%20Valid
          (Variables|Default|SetPlayer2 _returnvalue))
        (:Is%20Not%20Valid
          (Utilities|FlowControl|Delay 0.2)
          (goto _label_2))))))

(event Collision|EventActorBeginOverlap
  (params (OtherActor :type Actor%20Object%20Reference)))

(event EventTick
  (params (DeltaSeconds :type Float%20%28single-precision%29))
  (bind _self self)
  (bind _self_2 self)
  (bind _player1 (Variables|Default|GetPlayer1))
  (bind _player2 (Variables|Default|GetPlayer2))
  (bind _springarm (Variables|Default|GetSpringArm))
  (bind _returnvalue (Transformation|GetActorLocation _self))
  (bind _returnvalue_2 (Transformation|GetActorLocation _self_2))
  (bind _returnvalue_3 (Transformation|GetActorLocation _player1))
  (bind _returnvalue_4 (Transformation|GetActorLocation _player2))
  (bind _returnvalue_5 (Math|Vector|Distance(Vector) _returnvalue _returnvalue_3))
  (bind _returnvalue_6 (Math|Vector|Distance(Vector) _returnvalue_2 _returnvalue_4))
  (if (and (Utilities|IsValid (Variables|Default|GetPlayer2)) (Utilities|IsValid (Variables|Default|GetPlayer1)))
    (if (and (or (> _returnvalue_5 1e+02) (> _returnvalue_6 1e+02)) (or (< (Math|Vector|Distance(Vector) (Transformation|GetActorLocation self) (Transformation|GetActorLocation (Variables|Default|GetPlayer1))) 9e+02) (< (Math|Vector|Distance(Vector) (Transformation|GetActorLocation self) (Transformation|GetActorLocation (Variables|Default|GetPlayer2))) 9e+02)))
      (Variables|/Script/Engine.SpringArmComponent|SetTargetArmLength _springarm (Math|Interpolation|FInterpTo (Variables|/Script/Engine.SpringArmComponent|GetTargetArmLength _springarm) (* (+ _returnvalue_6 _returnvalue_5) 1.7) (Utilities|Time|GetWorldDeltaSeconds) 0.9)))))

(fn ConstructionScript)